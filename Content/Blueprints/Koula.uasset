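; Player-controlled rolling ball that restarts the current level when it takes damage.
; ForwardBack and LeftRight axis inputs apply torque to the physics sphere around its Y and X axes.
; Any damage triggers, only once, a camera fade-out held during a short delay before the level reloads.
; ChangeCameraView02 lets a caller set the spring arm's length, pitch and yaw to change the camera view.
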(event EventBeginPlay)

(event Collision|EventActorBeginOverlap
  (params (OtherActor :type Actor%20Object%20Reference)))

(event EventTick
  (params (DeltaSeconds :type Float%20%28single-precision%29)))

(event Game|Damage|EventAnyDamage
  (params (Damage :type Float%20%28single-precision%29) (DamageType :type Damage%20Type%20Object%20Reference) (InstigatedBy :type Controller%20Object%20Reference) (DamageCauser :type Actor%20Object%20Reference))
  (Utilities|FlowControl|DoOnce false
    (:Completed
      (CameraFades|StartCameraFade :self (Game|GetPlayerCameraManager 0) :ToAlpha 1.0 :Duration (Math|Float|MakeLiteralFloat 0.5) :bHoldWhenFinished true)
      (Utilities|FlowControl|Delay 0.5)
      (bind _returnvalue (Game|GetCurrentLevelName true))
      (Game|OpenLevel(byName) (Utilities|String|StringToName _returnvalue)))))

(event Input|AxisEvents|InputAxisForwardBack
  (params (AxisValue :type Float%20%28single-precision%29))
  (Class|PrimitiveComponent|AddTorqueinRadians (Variables|Default|GetSphere) (Math|Vector|MakeVector 0.0 (* AxisValue 1e+01) 0.0) "None" false))

(event Input|AxisEvents|InputAxisLeftRight
  (params (AxisValue :type Float%20%28single-precision%29))
  (Class|PrimitiveComponent|AddTorqueinRadians (Variables|Default|GetSphere) (Math|Vector|MakeVector (* AxisValue 1e+01) 0.0 0.0) "None" false))

(fn ConstructionScript)

(fn ChangeCameraView02
  (params (CameraDistance :type Float%20%28single-precision%29) (CameraRotationY :type Float%20%28single-precision%29) (CameraRoationZ :type Float%20%28single-precision%29))
  (bind _springarm (Variables|Default|GetSpringArm))
  (Variables|/Script/Engine.SpringArmComponent|SetTargetArmLength _springarm CameraDistance)
  (Transformation|SetRelativeRotation _springarm (Math|Rotator|MakeRotator 0.0 CameraRotationY CameraRoationZ) false false))