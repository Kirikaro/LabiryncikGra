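; Victory-area volume that completes the level when player pawn 0 enters its box with no Znajdźka (collectible) actors remaining.
; If any remain, it only prints a debug string.
; Completion looks up the current level name in the LevelNames array, then opens the next entry or quits the game on the last one.
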(event OnComponentBeginOverlap(Box)
  (params (OverlappedComponent :type Primitive%20Component%20Object%20Reference) (OtherActor :type Actor%20Object%20Reference) (OtherComp :type Primitive%20Component%20Object%20Reference) (OtherBodyIndex :type Integer) (bFromSweep :type Boolean) (SweepResult :type Hit%20Result%20Structure%20%28by%20ref%29))
  (if (== OtherActor (Game|Player|GetPlayerPawn 0))
    (bind _outactors (Actor|GetAllActorsOfClass "/Game/Blueprints/Znajdźka.Znajdźka_C"))
    (if (> (Utilities|Array|Length _outactors) 0)
      (Development|PrintString "Huj")
      (else
        (CallFunction|CompleteLvl)))))

(event EventBeginPlay)

(event Collision|EventActorBeginOverlap
  (params (OtherActor :type Actor%20Object%20Reference)))

(fn ConstructionScript)

(fn CompleteLvl
  (if (CallFunction|FinalLvl)
    (Game|QuitGame 0 "Quit" false)
    (else
      (CallFunction|LoadNextLvl))))

(fn GEtCurrentLvlIndex
  (bind _returnvalue (Game|GetCurrentLevelName true))
  (return (Utilities|Array|FindItem (Variables|Default|GetLevel%20names) _returnvalue)))

(fn GetCurrentLevelName)

(fn FinalLvl
  (return (== (Utilities|Array|LastIndex (Variables|Default|GetLevel%20names)) (CallFunction|GEtCurrentLvlIndex))))

(fn LoadNextLvl
  (Game|OpenLevel(byName) (Utilities|String|StringToName (CallFunction|GetNextLevelName))))

(fn GetNextLevelName
  (return (Utilities|Array|Get(acopy) (Variables|Default|GetLevel%20names) (+ (CallFunction|GEtCurrentLvlIndex) 1))))