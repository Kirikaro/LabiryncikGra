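; Collectible pickup actor ("Znajdźka") that reacts when the player pawn overlaps its sphere collision.
; After a short delay it plays a 2D sound and runs the CylinderMovement timeline.
; The timeline pulls the actor toward the player's current location, shrinks it to zero scale and drives the cylinder light's intensity down from full to zero by curve.
; The actor destroys itself when the timeline finishes.
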(event OnComponentBeginOverlap(Spherecollision)
  (params (OverlappedComponent :type Primitive%20Component%20Object%20Reference) (OtherActor :type Actor%20Object%20Reference) (OtherComp :type Primitive%20Component%20Object%20Reference) (OtherBodyIndex :type Integer) (bFromSweep :type Boolean) (SweepResult :type Hit%20Result%20Structure%20%28by%20ref%29))
  (if (== (Game|Player|GetPlayerPawn 0) OtherActor)
    (Utilities|FlowControl|Delay 0.2)
    (Audio|SpawnSound2D 0 1.0 1.0 0.0 0)
    (bind (_direction _cylindermove _scale _migniecia) (Timeline|CylinderMovement Play)
      (:Update
        (Transformation|SetActorLocation (Math|Vector|Lerp(Vector) (Transformation|GetActorLocation) (Transformation|GetActorLocation (Game|Player|GetPlayerPawn 0)) _cylindermove) false false)
        (Transformation|SetActorScale3D (Math|Vector|Lerp(Vector) (Transformation|GetActorScale3D) "0, 0, 0" _scale))
        (Rendering|Components|Light|SetIntensity (Variables|Default|GetCylinderLight) (Math|Float|Lerp 2e+04 0.0 _migniecia)))
      (:Finished
        (Actor|DestroyActor)))
    (else
      (Development|PrintString ""))))

(event Custom|CustomEvent
  (params (OverlappedComponent :type Primitive%20Component%20Object%20Reference) (OtherActor :type Actor%20Object%20Reference) (OtherComp :type Primitive%20Component%20Object%20Reference) (OtherBodyIndex :type Integer) (bFromSweep :type Boolean) (SweepResult :type Hit%20Result%20Structure%20%28by%20ref%29))
  (if (== (Game|Player|GetPlayerPawn 0) OtherActor)
    _))

(event EventBeginPlay)

(event EventTick
  (params (DeltaSeconds :type Float%20%28single-precision%29)))

(fn ConstructionScript)